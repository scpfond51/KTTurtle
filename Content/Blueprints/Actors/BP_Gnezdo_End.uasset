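; BP_Gnezdo_End is a numbered end-point actor for a "Gnezdo" (nest or socket) that records its own world location when selected.
; On BeginPlay it switches on ClickedSawn from WBPUIGnezdo and, if that matches its NumberOfEndGnezdo, saves its location to VectorToThisGnezdo.
; Indices 0 and 1 also copy it to Vector, while index 2 does not.
; The selection is read only at BeginPlay.
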(event EventBeginPlay
  (bind _numberofendgnezdo (Variables|Default|GetNumberOfEndGnezdo))
  (|CallParentFunction)
  (switch int (Variables|/Game/Blueprints/UI/WBP_UI.WBP_UI_C|GetClickedSawn (Variables|Default|GetWBP_UIGnezdo))
    (:0
      (if (== _numberofendgnezdo 0)
        (bind _returnvalue (Transformation|GetActorTransform))
        (bind _output_get (Variables|Default|SetVectorToThisGnezdo (.location _returnvalue)))
        (Variables|Default|SetVector _output_get)))
    (:1
      (if (== _numberofendgnezdo 1)
        (bind _returnvalue_2 (Transformation|GetActorTransform))
        (bind _output_get_2 (Variables|Default|SetVectorToThisGnezdo (.location _returnvalue_2)))
        (Variables|Default|SetVector _output_get_2)))
    (:2
      (if (== _numberofendgnezdo 2)
        (bind _returnvalue_3 (Transformation|GetActorTransform))
        (Variables|Default|SetVectorToThisGnezdo (.location _returnvalue_3))))))

(fn ConstructionScript
  (|CallParentFunction))