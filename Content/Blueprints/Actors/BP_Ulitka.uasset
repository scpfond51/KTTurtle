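; BP_Ulitka is a snail (ulitka) actor that crawls toward its BPGnezdo nest and destroys itself on overlapping a nest flagged EndGnezdo.
; A looping timer refreshes the target from the nest's location, while Tick turns and moves the snail toward it.
; TypeOfMovement selects steady motion, stop-and-go bursts, or bursts alternating with world-X drift, using DoOnce and Delay toggles.
; It caches BP_Manager on BeginPlay without using it here.
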(event OnComponentBeginOverlap(Box)
  (params (OverlappedComponent :type Primitive%20Component%20Object%20Reference) (OtherActor :type Actor%20Object%20Reference) (OtherComp :type Primitive%20Component%20Object%20Reference) (OtherBodyIndex :type Integer) (bFromSweep :type Boolean) (SweepResult :type Hit%20Result%20Structure%20%28by%20ref%29))
  ;[0.15 0.15 0.15 0.5] RemoveObject
  (bind _asbp_gnezdo (Utilities|Casting|CastToBP_Gnezdo OtherActor))
  (if (Variables|/Game/Blueprints/Actors/BP_Gnezdo.BP_Gnezdo_C|GetEndGnezdo? _asbp_gnezdo)
    (Actor|DestroyActor)))

(event Custom|Move
  ;[0.15 0.15 0.15 0.5] ChangeLocation
  (bind _returnvalue (Transformation|GetActorLocation (Variables|Default|GetBP_Gnezdo)))
  (Variables|Default|SetTargetLocation _returnvalue))

(event EventTick
  (params (DeltaSeconds :type Float%20%28single-precision%29))
  (switch int (Variables|Default|GetTypeOfMovement)
    (:0
      ;[0.15 0.15 0.15 0.5] BaseMovement
      (CallFunction|Movement (Variables|Default|GetTargetLocation) DeltaSeconds))
    (:1
      ;[0.15 0.15 0.15 0.5] SecondMovement
      (if (Variables|Default|GetSecondMovementTimer)
        (CallFunction|Movement (Variables|Default|GetTargetLocation) DeltaSeconds)
        (Utilities|TimerOfSecondMovement)))
    (:2
      ;[0.15 0.15 0.15 0.5] BaseMovement
      (if (Variables|Default|GetThirdMovementTimer)
        (CallFunction|Movement (Variables|Default|GetTargetLocation) DeltaSeconds)
        (Utilities|FlowControl|DoOnce false :!label _label
          (:Completed
            (Utilities|FlowControl|Delay 1.0)
            (Variables|Default|SetThirdMovementTimer false)
            (goto _label_2 Reset)))
        (else
          (Transformation|AddActorWorldOffset "1.000000,0.000000,0.000000")
          (Utilities|FlowControl|DoOnce false :!label _label_2
            (:Completed
              (Utilities|FlowControl|Delay 0.5)
              (Variables|Default|SetThirdMovementTimer true)
              (goto _label Reset))))))))

(event EventBeginPlay
  (bind _returnvalue (Actor|GetActorOfClass "/Game/Blueprints/Actors/BP_Manager.BP_Manager_C"))
  (Variables|Default|SetBP_Manager _returnvalue)
  ;[0.15 0.15 0.15 0.5] ChangeLocation
  (Utilities|Time|SetTimerbyEvent (delegate Custom|Move) 0.1 true))

(fn ConstructionScript)

(fn Movement
  (params (Target :type Vector%20%28by%20ref%29) (B :type Float%20%28single-precision%29))
  (Transformation|SetActorRotation (Math|Rotator|FindLookatRotation (Transformation|GetActorLocation) Target))
  (Transformation|AddActorWorldOffset (* (Transformation|GetActorForwardVector) B "100.000000,100.000000,100.000000")))