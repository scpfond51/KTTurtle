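; BP_Gnezdo is a nest actor ("gnezdo") that spawns a BP_Ulitka (snail) at its own transform when the UI requests it.
; Shortly after BeginPlay, it binds its Spawn event to the WBPUI spawn dispatcher.
; Spawn acts only when the UI's ClickedSawn value, one of three indices, matches this nest's NumberOfBeginGnezdo, then records it in NumberOfGnezdo before spawning.
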(event Custom|Spawn
  (bind _numberofbegingnezdo (Variables|Default|GetNumberOfBeginGnezdo))
  (switch int (Variables|/Game/Blueprints/UI/WBP_UI.WBP_UI_C|GetClickedSawn (Variables|Default|GetWBP_UI))
    (:0
      (if (== _numberofbegingnezdo 0)
        (Variables|Default|SetNumberOfGnezdo 0)
        (Game|SpawnActorfromClass "/Game/Blueprints/Actors/BP_Ulitka.BP_Ulitka_C" (Transformation|GetActorTransform) "Undefined" "MultiplyWithRoot" 0 0 :!label _label)))
    (:1
      (if (== _numberofbegingnezdo 1)
        (Variables|Default|SetNumberOfGnezdo 1)
        (goto _label)))
    (:2
      (if (== _numberofbegingnezdo 2)
        (Variables|Default|SetNumberOfGnezdo 2)
        (goto _label)))))

(event EventBeginPlay
  (Utilities|FlowControl|Delay 0.2)
  (EventDispatchers|BindEventtoSpawnDispatcher (Variables|Default|GetWBP_UI) (delegate Custom|Spawn)))

(fn ConstructionScript)