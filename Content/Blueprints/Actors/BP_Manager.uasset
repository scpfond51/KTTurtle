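; BP_Manager is an actor that spawns BP_Ulitka (snail) actors between BP_Gnezdo (nest) points when the player uses the UI.
; On BeginPlay it creates WBP_UI, shows the mouse cursor and caches every nest in the level.
; The widget's spawn dispatcher supplies an ID: the snail spawns at that ID's non-end nest and receives the matching end nest's location as its TargetLocation.
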(event Custom|ButtonClicked
  (bind _wbp_ui (Variables|Default|GetWBP_UI))
  (bind _clickedsawn (Variables|/Game/Blueprints/UI/WBP_UI.WBP_UI_C|GetClickedSawn _wbp_ui))
  ;[0.15 0.15 0.15 0.5] Spawn
  (bind _returnvalue (CallFunction|SpawnDeterminant _clickedsawn))
  (bind _returnvalue_2 (Game|SpawnActorfromClass "/Game/Blueprints/Actors/BP_Ulitka.BP_Ulitka_C" _returnvalue "Undefined" "MultiplyWithRoot" 0 0))
  (bind _returnvalue_3 (CallFunction|SpawnEndDeterminant _clickedsawn))
  (Variables|/Game/Blueprints/Actors/BP_Ulitka.BP_Ulitka_C|SetTargetLocation _returnvalue_2 _returnvalue_3))

(event Custom|UI
  ;[0.15 0.15 0.15 0.5] UI
  (bind _returnvalue (Game|ConstructObjectfromClass "/Game/Blueprints/UI/WBP_UI.WBP_UI_C"))
  (EventDispatchers|BindEventtoSpawnDispatcher _returnvalue (delegate Custom|ButtonClicked))
  (bind _output_get (Variables|Default|SetWBP_UI _returnvalue))
  (UserInterface|Viewport|AddtoViewport _output_get 0)
  (Variables|/Script/Engine.PlayerController|SetbShowMouseCursor (Game|GetPlayerController 0) true))

(event Custom|GetActors
  ;[0.15 0.15 0.15 0.5] GetActors
  (bind _outactors (Actor|GetAllActorsOfClass "/Game/Blueprints/Actors/BP_Gnezdo.BP_Gnezdo_C"))
  (Variables|Default|SetBP_Gnezdo _outactors))

(event EventBeginPlay
  ;[0.15 0.15 0.15 0.5] EventBeginPlay
  (CallFunction|UI)
  (CallFunction|GetActors))

(fn ConstructionScript)

(fn SpawnDeterminant
  (params (ID= :type Integer))
  (for _array_element (Variables|Default|GetBP_Gnezdo)
    (if (and (== (Variables|/Game/Blueprints/Actors/BP_Gnezdo.BP_Gnezdo_C|GetID _array_element) ID=) (not (Variables|/Game/Blueprints/Actors/BP_Gnezdo.BP_Gnezdo_C|GetEndGnezdo? _array_element)))
      (return (Math|Conversions|ToTransform(Vector) (Transformation|GetActorLocation _array_element))))))

(fn SpawnEndDeterminant
  (params (ID= :type Integer))
  (for _array_element (Variables|Default|GetBP_Gnezdo)
    (if (and (== (Variables|/Game/Blueprints/Actors/BP_Gnezdo.BP_Gnezdo_C|GetID _array_element) ID=) (Variables|/Game/Blueprints/Actors/BP_Gnezdo.BP_Gnezdo_C|GetEndGnezdo? _array_element))
      (return (Transformation|GetActorLocation _array_element)))))